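; Kitchen stove Blueprint that toggles a burner on and off and heats cookable items placed in its fire.
; Each overlap on the Switch component flips the state, activating or deactivating the particle system and enabling or disabling the Firehitbox's collision, which starts disabled.
; Actors entering or leaving the Firehitbox get their fire flag set or cleared, for CookCutActorBP and Kettle actors only.
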(event OnComponentBeginOverlap(Firehitbox)
  (params (OverlappedComponent :type Primitive%20Component%20Object%20Reference) (OtherActor :type Actor%20Object%20Reference) (OtherComp :type Primitive%20Component%20Object%20Reference) (OtherBodyIndex :type Integer) (bFromSweep :type Boolean) (SweepResult :type Hit%20Result%20Structure%20%28by%20ref%29))
  (bind _ascook_cut_actor_bp (Utilities|Casting|CastToCookCutActorBP OtherActor)
    (:then
      (Variables|/Game/Blueprint/CookCutActorBP.CookCutActorBP_C|SetonFire _ascook_cut_actor_bp true))
    (:CastFailed
      (bind _askettle (Utilities|Casting|CastToKettle OtherActor))
      (Variables|/Game/Blueprint/Kettle.Kettle_C|SetIsOnFire _askettle true))))

(event OnComponentEndOverlap(Firehitbox)
  (params (OverlappedComponent :type Primitive%20Component%20Object%20Reference) (OtherActor :type Actor%20Object%20Reference) (OtherComp :type Primitive%20Component%20Object%20Reference) (OtherBodyIndex :type Integer))
  (bind _ascook_cut_actor_bp (Utilities|Casting|CastToCookCutActorBP OtherActor)
    (:then
      (Variables|/Game/Blueprint/CookCutActorBP.CookCutActorBP_C|SetonFire _ascook_cut_actor_bp false))
    (:CastFailed
      (bind _askettle (Utilities|Casting|CastToKettle OtherActor))
      (Variables|/Game/Blueprint/Kettle.Kettle_C|SetIsOnFire _askettle false))))

(event OnComponentBeginOverlap(Switch)
  (params (OverlappedComponent :type Primitive%20Component%20Object%20Reference) (OtherActor :type Actor%20Object%20Reference) (OtherComp :type Primitive%20Component%20Object%20Reference) (OtherBodyIndex :type Integer) (bFromSweep :type Boolean) (SweepResult :type Hit%20Result%20Structure%20%28by%20ref%29))
  (bind _firehitbox (Variables|Default|GetFirehitbox))
  (bind _particlesystem (Variables|Default|GetParticleSystem))
  (bind _output_get (Variables|Default|SetSwitchTimes (not (Variables|Default|GetSwitchTimes))))
  (if _output_get
    (Components|Activation|Activate _particlesystem false)
    (Collision|SetCollisionEnabled _firehitbox "QueryOnly")
    (Variables|Default|Seton true)
    (else
      (Components|Activation|Deactivate _particlesystem)
      (Collision|SetCollisionEnabled _firehitbox "NoCollision")
      (Variables|Default|Seton false))))

(event EventBeginPlay
  (Collision|SetCollisionEnabled (Variables|Default|GetFirehitbox) "NoCollision")
  (Collision|SetCollisionEnabled (Variables|Default|GetParticleSystem) "QueryAndPhysics"))

(event Collision|EventActorBeginOverlap
  (params (OtherActor :type Actor%20Object%20Reference)))

(fn ConstructionScript)