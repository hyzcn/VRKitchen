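; A carrot-material prop that the Baxter robot can pick up, a knife can slice, and fire can recolor.
; BeginPlay copies its static mesh into a procedural mesh with a dynamic material.
; Box overlap attaches that mesh to the robot's wrist; knife overlap slices it along the blade component's plane, making the new half physics-simulated and parenting the static mesh to it.
; While OnFire is set, Tick plays a timeline that drives the material's color.
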(event OnComponentBeginOverlap(ProceduralMesh)
  (params (OverlappedComponent :type Primitive%20Component%20Object%20Reference) (OtherActor :type Actor%20Object%20Reference) (OtherComp :type Primitive%20Component%20Object%20Reference) (OtherBodyIndex :type Integer) (bFromSweep :type Boolean) (SweepResult :type Hit%20Result%20Structure%20%28by%20ref%29))
  (Utilities|Casting|CastToknife_Blueprint OtherActor)
  (bind _outotherhalfprocmesh (Class|KismetProceduralMeshLibrary|SliceProceduralMesh (Variables|Default|GetProceduralMesh) (Transformation|GetWorldLocation OtherComp) (Math|Vector|GetUpVector OtherComp) true "CreateNewSectionForCap" "/Game/Scenes/Small_Items/Distractor/napkin/_Beige_1._Beige_1"))
  (bind _output_get (Variables|Default|SetSlicedProceduralMesh _outotherhalfprocmesh))
  (Physics|SetSimulatePhysics _output_get true)
  (Collision|SetCollisionEnabled _output_get "QueryAndPhysics")
  (Collision|SetCollisionResponsetoAllChannels _output_get "ECR_Block")
  (Class|PrimitiveComponent|SetNotifyRigidBodyCollision _output_get true)
  (Transformation|AttachComponentToComponent (Variables|Debug|GetStaticMeshComponent) _output_get "None" "KeepRelative" "KeepRelative" "KeepRelative" true))

(event OnComponentBeginOverlap(Box)
  (params (OverlappedComponent :type Primitive%20Component%20Object%20Reference) (OtherActor :type Actor%20Object%20Reference) (OtherComp :type Primitive%20Component%20Object%20Reference) (OtherBodyIndex :type Integer) (bFromSweep :type Boolean) (SweepResult :type Hit%20Result%20Structure%20%28by%20ref%29))
  (bind _asbaxter_robot (Utilities|Casting|CastToBaxterRobot OtherActor))
  (Transformation|AttachComponentToComponent (Variables|Default|GetProceduralMesh) (Variables|/Script/VRInteractPlatform.BaxterRobot|GetSM_RWrist _asbaxter_robot) "None" "KeepWorld" "KeepWorld" "KeepWorld" true))

(event EventBeginPlay
  (Class|KismetProceduralMeshLibrary|CopyProceduralMeshfromStaticMeshComponent (Variables|Debug|GetStaticMeshComponent) 0 (Variables|Default|GetProceduralMesh) true)
  (bind _returnvalue (Rendering|Material|CreateDynamicMaterialInstance (Variables|Default|GetProceduralMesh) 0 "/Game/Scenes/Other_Utilities/carrot/carrot_dynamic.carrot_dynamic" :!class /Script/Engine.PrimitiveComponent))
  (Variables|Default|SetonFire false))

(event Collision|EventActorBeginOverlap
  (params (OtherActor :type Actor%20Object%20Reference)))

(event EventTick
  (params (DeltaSeconds :type Float%20%28single-precision%29))
  (if (Variables|Default|GetonFire)
    (bind _newtrack_0 (Timeline|Timeline_0 Play)
      (:Update
        (Rendering|Material|SetVectorParameterValue (stale EventBeginPlay _returnvalue) "Color" _newtrack_0 :!class /Script/Engine.MaterialInstanceDynamic)))))

(fn ConstructionScript)