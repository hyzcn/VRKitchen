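; Kitchen knife actor that slices CookCutActorBP food when its invisible blade component overlaps one of that food's procedural meshes.
; It calls Slice on the food with a plane taken from the invisible knife's location and up vector.
; A "Skin" component tag separates skin from fruit, each with its own flag and half-second delay to block repeated cuts.
; Debug prints mark each cut, and the end-overlap event is empty.
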(event OnComponentBeginOverlap(Knife_invis)
  (params (OverlappedComponent :type Primitive%20Component%20Object%20Reference) (OtherActor :type Actor%20Object%20Reference) (OtherComp :type Primitive%20Component%20Object%20Reference) (OtherBodyIndex :type Integer) (bFromSweep :type Boolean) (SweepResult :type Hit%20Result%20Structure%20%28by%20ref%29))
  (bind _knife_invis (Variables|Default|GetKnife_invis))
  (bind _returnvalue (Transformation|GetWorldLocation _knife_invis))
  (bind _returnvalue_2 (Math|Vector|GetUpVector _knife_invis))
  (bind _asprocedural_mesh_component (Utilities|Casting|CastToProceduralMeshComponent OtherComp))
  (bind _ascook_cut_actor_bp (Utilities|Casting|CastToCookCutActorBP (Components|GetOwner _asprocedural_mesh_component)))
  (if (not (select (not (Components|ComponentHasTag _asprocedural_mesh_component "Skin")) (Variables|Default|GetSlicedFruit) (Variables|Default|GetSlicedSkin)))
    (if (not (Components|ComponentHasTag _asprocedural_mesh_component "Skin"))
      (Variables|Default|SetSlicedFruit true)
      (Development|PrintString "Fruit")
      (Default|Slice _ascook_cut_actor_bp _returnvalue _returnvalue_2 _asprocedural_mesh_component)
      (Utilities|FlowControl|Delay 0.5)
      (Variables|Default|SetSlicedFruit false)
      (else
        (Variables|Default|SetSlicedSkin true)
        (Development|PrintString "Skin")
        (Default|Slice _ascook_cut_actor_bp _returnvalue _returnvalue_2 _asprocedural_mesh_component)
        (Utilities|FlowControl|Delay 0.5)
        (Variables|Default|SetSlicedSkin false)))))

(event OnComponentEndOverlap(Knife_invis)
  (params (OverlappedComponent :type Primitive%20Component%20Object%20Reference) (OtherActor :type Actor%20Object%20Reference) (OtherComp :type Primitive%20Component%20Object%20Reference) (OtherBodyIndex :type Integer)))

(event EventBeginPlay)

(event Collision|EventActorBeginOverlap
  (params (OtherActor :type Actor%20Object%20Reference)))

(event EventTick
  (params (DeltaSeconds :type Float%20%28single-precision%29)))

(fn ConstructionScript)