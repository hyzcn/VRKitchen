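; JuicerBP is a kitchen juicer actor that turns cut, squeezable ingredients into juice.
; When a PickCookCutObject overlaps SqueezeBox with both CanSqueeze and Cut set, the juicer calls RecieveFluid with that object's SqueezeColor, adding a fixed amount of "Juice".
; Other overlapping actors are checked for spoon2, which only prints the current FluidColor.
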(event OnComponentBeginOverlap(SqueezeBox)
  (params (OverlappedComponent :type Primitive%20Component%20Object%20Reference) (OtherActor :type Actor%20Object%20Reference) (OtherComp :type Primitive%20Component%20Object%20Reference) (OtherBodyIndex :type Integer) (bFromSweep :type Boolean) (SweepResult :type Hit%20Result%20Structure%20%28by%20ref%29))
  (bind _aspick_cook_cut_object (Utilities|Casting|CastToPickCookCutObject OtherActor)
    (:then
      (if (and (Variables|/Script/VRInteractPlatform.PickCookCutObject|GetCanSqueeze _aspick_cook_cut_object) (Variables|/Script/VRInteractPlatform.PickCookCutObject|Getcut _aspick_cook_cut_object))
        (Class|PourContainer|RecieveFluid self (Variables|/Script/VRInteractPlatform.PickCookCutObject|GetSqueezeColor _aspick_cook_cut_object) 0.1 "Juice")))
    (:CastFailed
      (Utilities|Casting|CastTospoon2 OtherActor)
      (Development|PrintString (Utilities|String|ToString(Integer) (Variables|Default|GetFluidColor))))))

(event EventBeginPlay)

(event Collision|EventActorBeginOverlap
  (params (OtherActor :type Actor%20Object%20Reference)))

(event EventTick
  (params (DeltaSeconds :type Float%20%28single-precision%29))
  (|CallParentFunction DeltaSeconds))

(fn ConstructionScript
  (|CallParentFunction))