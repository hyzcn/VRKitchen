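; Saucepan actor that tracks which physics and world-dynamic components are currently inside it.
; Each Tick it clears ContainedObjects and runs a small, very short box multi-trace just below the static mesh's origin.
; The box follows the mesh's rotation with a 90-degree roll offset.
; Components from blocking hits are stored uniquely in ContainedObjects; this graph does nothing further with them.
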(event EventBeginPlay)

(event Collision|EventActorBeginOverlap
  (params (OtherActor :type Actor%20Object%20Reference)))

(event EventTick
  (params (DeltaSeconds :type Float%20%28single-precision%29))
  (bind _staticmeshcomponent (Variables|Default|GetStaticMeshComponent))
  (bind _returnvalue (Transformation|GetWorldRotation _staticmeshcomponent))
  (bind _returnvalue_2 (Transformation|GetWorldLocation _staticmeshcomponent))
  (bind (_roll _pitch _yaw) (Math|Rotator|BreakRotator _returnvalue))
  (bind _returnvalue_3 (+ _returnvalue_2 "0, 0,-2.500000"))
  (Utilities|Array|Clear (Variables|Default|GetContainedObjects))
  (bind _outhits (Class|KismetSystemLibrary|BoxTraceMultiforObjects _returnvalue_3 (+ _returnvalue_3 "0, 0,0.100000") "10.000000,10.000000,2.000000" (Math|Rotator|MakeRotator (+ _roll 9e+01) _pitch _yaw) (Utilities|Array|MakeArray "ObjectTypeQuery2" "ObjectTypeQuery4") false 0 "None" true))
  (for _array_element _outhits
    (if (.bBlockingHit (Collision|BreakHitResult _array_element))
      (Utilities|Array|AddUnique (Variables|Default|GetContainedObjects) (.HitComponent (Collision|BreakHitResult _array_element))))))

(fn ConstructionScript)