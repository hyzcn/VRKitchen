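; Knife Blueprint that cuts procedural mesh objects on robot pickup actors when it touches them.
; When its invisible Knife_invis component begins overlapping a procedural mesh owned by a robot_pickup_Blueprint, it calls that actor's Slice function.
; The cut plane comes from the invisible blade's world location and up vector.
; A Sliced flag with a short delay acts as a cooldown against repeated cuts.
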(event OnComponentBeginOverlap(Knife_invis)
  (params (OverlappedComponent :type Primitive%20Component%20Object%20Reference) (OtherActor :type Actor%20Object%20Reference) (OtherComp :type Primitive%20Component%20Object%20Reference) (OtherBodyIndex :type Integer) (bFromSweep :type Boolean) (SweepResult :type Hit%20Result%20Structure%20%28by%20ref%29))
  (bind _knife_invis (Variables|Default|GetKnife_invis))
  (bind _asprocedural_mesh_component (Utilities|Casting|CastToProceduralMeshComponent OtherComp))
  (bind _asrobot_pickup_blueprint (Utilities|Casting|CastTorobot_pickup_Blueprint (Components|GetOwner _asprocedural_mesh_component)))
  (if (not (Variables|Default|GetSliced))
    (Default|Slice _asrobot_pickup_blueprint (Transformation|GetWorldLocation _knife_invis) (Math|Vector|GetUpVector _knife_invis) _asprocedural_mesh_component)
    (Variables|Default|SetSliced true)
    (Utilities|FlowControl|Delay 1.0)
    (Variables|Default|SetSliced false)))

(event EventBeginPlay)

(event Collision|EventActorBeginOverlap
  (params (OtherActor :type Actor%20Object%20Reference)))

(event EventTick
  (params (DeltaSeconds :type Float%20%28single-precision%29)))

(fn ConstructionScript)