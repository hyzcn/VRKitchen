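; Spoon actor for a kitchen game that scoops solid food or liquid when its ContainerMesh stops overlapping a source.
; Leaving a spoonable PickCookCutObject attaches a Cylinder wearing that food's material as a stand-in portion.
; Leaving the FillMesh of another non-empty PourContainer receives a small amount of its fluid.
; Tick watches the Drop flag, then detaches a held solid with physics and collision enabled.
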(event OnComponentEndOverlap(ContainerMesh)
  (params (OverlappedComponent :type Primitive%20Component%20Object%20Reference) (OtherActor :type Actor%20Object%20Reference) (OtherComp :type Primitive%20Component%20Object%20Reference) (OtherBodyIndex :type Integer))
  (bind _cylinder (Variables|Default|GetCylinder))
  ;[1 1 1] Solid
  (bind _aspick_cook_cut_object (Utilities|Casting|CastToPickCookCutObject OtherActor)
    (:then
      (if (Variables|/Script/VRInteractPlatform.PickCookCutObject|GetSpoon _aspick_cook_cut_object)
        (if (not (Variables|Default|Getstuffed))
          (bind _returnvalue (Rendering|Material|CreateDynamicMaterialInstance _cylinder 0 (Rendering|Material|GetMaterial (Variables|/Script/Engine.StaticMeshComponent|GetStaticMesh (Variables|/Script/Engine.StaticMeshActor|GetStaticMeshComponent _aspick_cook_cut_object)) 0) :!class /Script/Engine.PrimitiveComponent))
          (Rendering|Material|SetScalarParameterValue _returnvalue "opacity" 1.0 :!class /Script/Engine.MaterialInstanceDynamic)
          (Transformation|SetRelativeLocationAndRotation _cylinder "0.040000,-0.137000,-1.660000" "0, 0,-90.000000" false false)
          (Transformation|AttachComponentToComponent _cylinder (Variables|Default|GetContainerMesh) "None" "KeepRelative" "KeepRelative" "KeepWorld" true)
          (Variables|Default|Setstuffed true)
          (Variables|Default|Setsolid true))))
    (:CastFailed
      ;[1 1 1] liquid
      (bind _aspour_container (Utilities|Casting|CastToPourContainer OtherActor))
      (if (and (> (Variables|/Script/VRInteractPlatform.PourContainer|GetCurrentFillFraction _aspour_container) 0.0) (and (Utilities|Enum|Equal(Enum) (Utilities|GetObjectName OtherComp) "FillMesh") (!= OtherActor self)))
        (Variables|Default|Setstuffed true)
        (Class|PourContainer|RecieveFluid (Variables|/Script/VRInteractPlatform.PourContainer|GetFluidColor _aspour_container) 0.02 (Variables|/Script/VRInteractPlatform.PourContainer|GetFluidName _aspour_container))))))

(event EventTick
  (params (DeltaSeconds :type Float%20%28single-precision%29))
  (bind _cylinder (Variables|Default|GetCylinder))
  ;[1 1 1] drop object
  (if (Math|Boolean|ANDBoolean (Variables|Default|GetDrop) (Variables|Default|Getsolid) (Variables|Default|Getstuffed))
    (Transformation|DetachFromComponent _cylinder "KeepWorld" "KeepWorld" "KeepWorld" true)
    (Collision|SetCollisionResponsetoChannel (Variables|Default|GetCylinder) "ECC_WorldDynamic" "ECR_Block")
    (Physics|SetSimulatePhysics _cylinder true)
    (Variables|Default|Setstuffed false)
    (Variables|Default|SetDrop false)
    (Variables|Default|Setsolid false)))

(fn ConstructionScript)