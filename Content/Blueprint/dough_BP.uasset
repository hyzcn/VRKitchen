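; Dough actor that changes into an expanded shape when it hits something while moving fast enough.
; On each component hit, it compares the static mesh's physics linear velocity against a minimum speed and, if met, swaps in the expanded dough mesh.
; An Expand flag, cleared at BeginPlay, makes the swap a one-time change with no way back.
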(event OnComponentHit(StaticMeshComponent)
  (params (HitComponent :type Primitive%20Component%20Object%20Reference) (OtherActor :type Actor%20Object%20Reference) (OtherComp :type Primitive%20Component%20Object%20Reference) (NormalImpulse :type Vector :default "0, 0, 0") (Hit :type Hit%20Result%20Structure%20%28by%20ref%29))
  (if (not (Variables|Default|GetExpand))
    (bind _returnvalue (Physics|GetPhysicsLinearVelocity (Variables|Debug|GetStaticMeshComponent) "None"))
    (if (>= (Math|Vector|VectorLength _returnvalue) 1e+02)
      (Components|StaticMesh|SetStaticMesh (Variables|Debug|GetStaticMeshComponent) "/Game/Assets/pizza_dough/dough_expand.dough_expand")
      (Variables|Default|SetExpand true))))

(event EventBeginPlay
  (Variables|Default|SetExpand false))

(event Collision|EventActorBeginOverlap
  (params (OtherActor :type Actor%20Object%20Reference)))

(event EventTick
  (params (DeltaSeconds :type Float%20%28single-precision%29)))

(fn ConstructionScript)