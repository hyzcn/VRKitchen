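; A cookable, sliceable food actor that can be cut into physics pieces and changes color while on fire.
; BeginPlay copies the static mesh into a procedural mesh, with an optional dynamic material whose color a timeline animates before flagging it cooked.
; Slice cuts fruit with a cap material and "Skin"-tagged components without caps.
; New skin halves attach to their saved fruit halves, with collision adjusted between them.
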(event EventBeginPlay
  (bind _fruit (Variables|Default|GetFruit))
  (Variables|Default|SetonFire false)
  (Class|KismetProceduralMeshLibrary|CopyProceduralMeshfromStaticMeshComponent (Variables|Default|GetStaticMeshComponent) 0 _fruit true)
  (Rendering|Material|SetMaterial _fruit 0 (Variables|Default|GetSourceMat))
  (Utilities|Array|Add (Variables|Default|GetProcMeshes) _fruit)
  (if (Variables|Default|GetChangeColor)
    (bind _returnvalue (Rendering|Material|CreateDynamicMaterialInstance (Variables|Default|GetFruit) 0 (Variables|Default|GetSourceMat) :!class /Script/Engine.PrimitiveComponent))))

(event Collision|EventActorBeginOverlap
  (params (OtherActor :type Actor%20Object%20Reference)))

(event EventTick
  (params (DeltaSeconds :type Float%20%28single-precision%29))
  (if (Variables|Default|GetonFire)
    (bind _newtrack_0 (Timeline|Timeline_0 Play)
      (:Update
        (Rendering|Material|SetVectorParameterValue (stale EventBeginPlay _returnvalue) "Color" _newtrack_0 :!class /Script/Engine.MaterialInstanceDynamic))
      (:Finished
        (Variables|Default|Setcook true)))))

(fn ConstructionScript)

(fn Slice
  (params (Position :type Vector) (Normal :type Vector) (ComponentToSlice :type Procedural%20Mesh%20Component%20Object%20Reference))
  (bind _returnvalue (Components|ComponentHasTag ComponentToSlice "Skin"))
  (bind _outotherhalfprocmesh (Class|KismetProceduralMeshLibrary|SliceProceduralMesh ComponentToSlice Position Normal true (select _returnvalue "NoCap" "CreateNewSectionForCap") (Variables|Default|GetCapMat)))
  (if _returnvalue
    (bind _output_get (Variables|Default|SetSavedSkin _outotherhalfprocmesh))
    (Variables|/Script/Engine.ActorComponent|SetComponentTags _output_get (Variables|/Script/Engine.ActorComponent|GetComponentTags ComponentToSlice))
    (Collision|SetCollisionObjectType _output_get "ECC_Destructible")
    (Physics|SetSimulatePhysics _output_get false)
    (if (Variables|Default|GetSavedFruitSet)
      (Transformation|AttachComponentToComponent _output_get (Variables|Default|GetSavedFruit) "None" "KeepWorld" "KeepWorld" "KeepWorld" false)
      (Collision|SetCollisionResponsetoChannel (stale _output_get_2) "ECC_Destructible" "ECR_Ignore")
      (Collision|SetCollisionEnabled (stale _output_get_2) "QueryAndPhysics")
      (Physics|SetSimulatePhysics (stale _output_get_2) true)
      (Variables|Default|Setcut true)
      (Variables|Default|SetSavedFruitSet false))
    (else
      (bind _output_get_2 (Variables|Default|SetSavedFruit _outotherhalfprocmesh))
      (Variables|Default|SetSavedFruitSet true)
      (Variables|/Script/Engine.ActorComponent|SetComponentTags _output_get_2 (Variables|/Script/Engine.ActorComponent|GetComponentTags ComponentToSlice))
      (Collision|SetCollisionObjectType _output_get_2 "ECC_WorldDynamic")
      (if (> (Utilities|Array|Length (Actor|GetComponentsbyTag self "/Script/ProceduralMeshComponent.ProceduralMeshComponent" "Skin")) 0)
        (Collision|SetCollisionEnabled _output_get_2 "NoCollision")
        (else
          (Physics|SetSimulatePhysics _output_get_2 true))))))