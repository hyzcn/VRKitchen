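; Blender actor for a cooking game that turns squeezable cut ingredients into fluid inside a pour container.
; Its Box overlap stores an open container that can receive fluid and clears that reference when it leaves.
; When a squeezable CookCutActorBP enters while a container is stored, it destroys the overlapped mesh and adds a fixed amount of "Blending" fluid, colored halfway between the container's and ingredient's colors.
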(event OnComponentBeginOverlap(Box)
  (params (OverlappedComponent :type Primitive%20Component%20Object%20Reference) (OtherActor :type Actor%20Object%20Reference) (OtherComp :type Primitive%20Component%20Object%20Reference) (OtherBodyIndex :type Integer) (bFromSweep :type Boolean) (SweepResult :type Hit%20Result%20Structure%20%28by%20ref%29))
  (bind _asbp_pour_container (Utilities|Casting|CastToBP_PourContainer OtherActor)
    (:then
      (if (and (Variables|/Script/VRInteractPlatform.PourContainer|GetCanReceiveFluid _asbp_pour_container) (Variables|/Script/VRInteractPlatform.PourContainer|GetOpen _asbp_pour_container))
        (Variables|Default|SetContainerRef _asbp_pour_container)))
    (:CastFailed
      (bind _ascook_cut_actor_bp (Utilities|Casting|CastToCookCutActorBP OtherActor))
      (if (and (Variables|/Script/VRInteractPlatform.PickCookCutObject|GetCanSqueeze _ascook_cut_actor_bp) (Utilities|IsValid (Variables|Default|GetContainerRef)))
        (Default|DestroyMesh _ascook_cut_actor_bp OtherComp)
        (Class|PourContainer|RecieveFluid (Variables|Default|GetContainerRef) (Math|Color|Lerp(LinearColor) (Variables|/Script/VRInteractPlatform.PourContainer|GetFluidColor (Variables|Default|GetContainerRef)) (Variables|/Script/VRInteractPlatform.PickCookCutObject|GetSqueezeColor _ascook_cut_actor_bp) 0.5) 0.1 "Blending")))))

(event OnComponentEndOverlap(Box)
  (params (OverlappedComponent :type Primitive%20Component%20Object%20Reference) (OtherActor :type Actor%20Object%20Reference) (OtherComp :type Primitive%20Component%20Object%20Reference) (OtherBodyIndex :type Integer))
  (bind _asbp_pour_container (Utilities|Casting|CastToBP_PourContainer OtherActor))
  (if (== _asbp_pour_container (Variables|Default|GetContainerRef))
    (Variables|Default|SetContainerRef 0)))

(event EventBeginPlay)

(event Collision|EventActorBeginOverlap
  (params (OtherActor :type Actor%20Object%20Reference)))

(event EventTick
  (params (DeltaSeconds :type Float%20%28single-precision%29)))

(fn ConstructionScript)