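; Mainframe actor that keeps track of the objects sitting within a box volume at its location.
; Every Tick it clears ContainedObjects and runs a short multi box trace for WorldDynamic and PhysicsBody objects.
; Components from blocking hits are added uniquely, so the list holds components rather than actors and is rebuilt each frame.
; Nothing in this Blueprint reads the list.
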(event EventBeginPlay)

(event Collision|EventActorBeginOverlap
  (params (OtherActor :type Actor%20Object%20Reference)))

(event EventTick
  (params (DeltaSeconds :type Float%20%28single-precision%29))
  (bind _returnvalue (Transformation|GetActorLocation))
  (Utilities|Array|Clear (Variables|Default|GetContainedObjects))
  (bind _outhits (Class|KismetSystemLibrary|BoxTraceMultiforObjects _returnvalue (+ (+ _returnvalue "0,5.000000,5.000000") "0, 0,0.100000") "47.000000,22.000000,32.000000" "0, 0, 0" (Utilities|Array|MakeArray "ObjectTypeQuery2" "ObjectTypeQuery4") false 0 "None" true))
  (for _array_element _outhits
    (if (.bBlockingHit (Collision|BreakHitResult _array_element))
      (Utilities|Array|AddUnique (Variables|Default|GetContainedObjects) (.HitComponent (Collision|BreakHitResult _array_element))))))

(fn ConstructionScript)