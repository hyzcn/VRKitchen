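; Peelable fruit actor whose skin can be sliced off in pieces.
; On BeginPlay it copies a static mesh into the procedural Skin mesh with collision and tracks it in ProcMeshes.
; Peel and PeelNew slice a skin component along a plane without caps, free one half to simulate physics and re-attach the other to Fruit as Destructible.
; The two functions differ in which half is released.
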(event EventBeginPlay
  (bind _skin (Variables|Default|GetSkin))
  (|CallParentFunction)
  (Class|KismetProceduralMeshLibrary|CopyProceduralMeshfromStaticMeshComponent (Variables|Default|GetStaticMeshComponent) 0 _skin true)
  (Utilities|Array|Add (Variables|Default|GetProcMeshes) _skin))

(event Collision|EventActorBeginOverlap
  (params (OtherActor :type Actor%20Object%20Reference))
  (|CallParentFunction OtherActor))

(event EventTick
  (params (DeltaSeconds :type Float%20%28single-precision%29))
  (|CallParentFunction DeltaSeconds))

(fn ConstructionScript
  (|CallParentFunction))

(fn Peel
  (params (Position :type Vector) (Normal :type Vector) (ComponentToPeel :type Procedural%20Mesh%20Component%20Object%20Reference))
  (bind _fruit (Variables|Default|GetFruit))
  (bind _outotherhalfprocmesh (Class|KismetProceduralMeshLibrary|SliceProceduralMesh ComponentToPeel Position Normal true "NoCap"))
  (Variables|Default|SetSlicedProceduralMesh _outotherhalfprocmesh)
  (Utilities|Array|Add (Variables|Default|GetProcMeshes) (Variables|Default|GetSlicedProceduralMesh))
  (Physics|SetSimulatePhysics ComponentToPeel true)
  (Collision|SetCollisionObjectType (Variables|Default|GetSlicedProceduralMesh) "ECC_Destructible")
  (Physics|SetSimulatePhysics (Variables|Default|GetSlicedProceduralMesh) false)
  (Transformation|AttachComponentToComponent (Variables|Default|GetSlicedProceduralMesh) _fruit "None" "KeepRelative" "KeepRelative" "KeepRelative" false)
  (Transformation|SetWorldTransform (Variables|Default|GetSlicedProceduralMesh) (Transformation|GetWorldTransform _fruit) false false))

(fn PeelNew
  (params (Position :type Vector) (Normal :type Vector) (ComponentToPeel :type Procedural%20Mesh%20Component%20Object%20Reference))
  (bind _fruit (Variables|Default|GetFruit))
  (bind _outotherhalfprocmesh (Class|KismetProceduralMeshLibrary|SliceProceduralMesh ComponentToPeel Position Normal true "NoCap"))
  (bind _output_get (Variables|Default|SetSlicedProceduralMesh _outotherhalfprocmesh))
  (Utilities|Array|Add (Variables|Default|GetProcMeshes) 0)
  (Physics|SetSimulatePhysics _output_get true)
  (Collision|SetCollisionObjectType ComponentToPeel "ECC_Destructible")
  (Physics|SetSimulatePhysics ComponentToPeel false)
  (Transformation|AttachComponentToComponent ComponentToPeel _fruit "None" "KeepRelative" "KeepRelative" "KeepRelative" false)
  (Transformation|SetWorldTransform ComponentToPeel (Transformation|GetWorldTransform _fruit) false false))