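; CanBP is an openable can whose lid is split into four quarters that a CanOpenerBP cuts one by one.
; When the opener ends overlap with a quarter, that quarter swaps to a flipped mesh and sets its flag.
; Tick polls the four flags and, once all are set, disables quarter collision, hides the Scene hierarchy and shows Top as a physics-simulated piece.
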(event OnComponentEndOverlap(lid2)
  (params (OverlappedComponent :type Primitive%20Component%20Object%20Reference) (OtherActor :type Actor%20Object%20Reference) (OtherComp :type Primitive%20Component%20Object%20Reference) (OtherBodyIndex :type Integer))
  (Utilities|Casting|CastToCanOpenerBP OtherActor)
  (Components|StaticMesh|SetStaticMesh (Variables|Default|Getlid2) "/Game/Assets/can/lid_quarter_flip.lid_quarter_flip")
  (Variables|Default|Setflipped2 true))

(event OnComponentEndOverlap(lid3)
  (params (OverlappedComponent :type Primitive%20Component%20Object%20Reference) (OtherActor :type Actor%20Object%20Reference) (OtherComp :type Primitive%20Component%20Object%20Reference) (OtherBodyIndex :type Integer))
  (Utilities|Casting|CastToCanOpenerBP OtherActor)
  (Components|StaticMesh|SetStaticMesh (Variables|Default|Getlid3) "/Game/Assets/can/lid_quarter_flip.lid_quarter_flip")
  (Variables|Default|Setflipped3 true))

(event OnComponentEndOverlap(lid1)
  (params (OverlappedComponent :type Primitive%20Component%20Object%20Reference) (OtherActor :type Actor%20Object%20Reference) (OtherComp :type Primitive%20Component%20Object%20Reference) (OtherBodyIndex :type Integer))
  (Utilities|Casting|CastToCanOpenerBP OtherActor)
  (Components|StaticMesh|SetStaticMesh (Variables|Default|Getlid1) "/Game/Assets/can/lid_quarter_flip.lid_quarter_flip")
  (Variables|Default|Setflipped1 true))

(event OnComponentEndOverlap(lid4)
  (params (OverlappedComponent :type Primitive%20Component%20Object%20Reference) (OtherActor :type Actor%20Object%20Reference) (OtherComp :type Primitive%20Component%20Object%20Reference) (OtherBodyIndex :type Integer))
  (Utilities|Casting|CastToCanOpenerBP OtherActor)
  (Components|StaticMesh|SetStaticMesh (Variables|Default|Getlid4) "/Game/Assets/can/lid_quarter_flip.lid_quarter_flip")
  (Variables|Default|Setflipped4 true))

(event EventBeginPlay)

(event Collision|EventActorBeginOverlap
  (params (OtherActor :type Actor%20Object%20Reference)))

(event EventTick
  (params (DeltaSeconds :type Float%20%28single-precision%29))
  (bind _top (Variables|Default|Gettop))
  (if (and (and (Variables|Default|Getflipped1) (Variables|Default|Getflipped2)) (and (Variables|Default|Getflipped3) (Variables|Default|Getflipped4)))
    (Collision|SetCollisionEnabled (Variables|Default|Getlid1) "NoCollision")
    (Collision|SetCollisionEnabled (Variables|Default|Getlid2) "NoCollision")
    (Collision|SetCollisionEnabled (Variables|Default|Getlid3) "NoCollision")
    (Collision|SetCollisionEnabled (Variables|Default|Getlid4) "NoCollision")
    (Rendering|SetVisibility (Variables|Default|GetScene) false true)
    (Rendering|SetVisibility _top true false)
    (Collision|SetCollisionEnabled _top "QueryAndPhysics")
    (Physics|SetSimulatePhysics _top true)))

(fn ConstructionScript)