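; Kettle Blueprint that starts boiling after it has been on fire for more than five seconds in total.
; Tick adds elapsed time to Temperature while IsOnFire is true, then sets IsBoiling and activates the particle system past the threshold.
; When the fire is off, boiling and particles stop, but Temperature keeps its value, resetting only on BeginPlay.
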(event EventBeginPlay
  (Variables|Default|SetTemperature 0.0))

(event Collision|EventActorBeginOverlap
  (params (OtherActor :type Actor%20Object%20Reference)))

(event EventTick
  (params (DeltaSeconds :type Float%20%28single-precision%29))
  (if (Variables|Default|GetIsOnFire)
    (bind _output_get (Variables|Default|SetTemperature (+ (Variables|Default|GetTemperature) DeltaSeconds)))
    (if (> _output_get 5.0)
      (Variables|Default|SetIsBoiling true)
      (Components|Activation|Activate (Variables|Default|GetParticleSystem) false))
    (else
      (Variables|Default|SetIsBoiling false)
      (Components|Activation|Deactivate (Variables|Default|GetParticleSystem)))))

(fn ConstructionScript
  (|CallParentFunction))