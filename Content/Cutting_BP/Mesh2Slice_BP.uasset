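; Sliceable mesh actor that a knife_Blueprint can cut in two.
; On BeginPlay it copies its static mesh component Mesh2Slice into a ProceduralMesh component with collision.
; When a knife overlaps that mesh, SliceProceduralMesh cuts it on a plane taken from the overlapping component's location and up vector, caps the cut and enables physics on the new half, with debug prints.
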(event OnComponentBeginOverlap(ProceduralMesh)
  (params (OverlappedComponent :type Primitive%20Component%20Object%20Reference) (OtherActor :type Actor%20Object%20Reference) (OtherComp :type Primitive%20Component%20Object%20Reference) (OtherBodyIndex :type Integer) (bFromSweep :type Boolean) (SweepResult :type Hit%20Result%20Structure%20%28by%20ref%29))
  (Utilities|Casting|CastToknife_Blueprint OtherActor)
  (Development|PrintString "Overlap!!!")
  (bind _outotherhalfprocmesh (Class|KismetProceduralMeshLibrary|SliceProceduralMesh (Variables|Default|GetProceduralMesh) (Transformation|GetWorldLocation OtherComp) (Math|Vector|GetUpVector OtherComp) true "CreateNewSectionForCap" "/Engine/MapTemplates/Materials/BasicAsset01.BasicAsset01"))
  (bind _output_get (Variables|Default|SetSlicedProceduralMesh _outotherhalfprocmesh))
  (Physics|SetSimulatePhysics _output_get true)
  (Development|PrintString "Sliced!!!"))

(event EventBeginPlay
  (Class|KismetProceduralMeshLibrary|CopyProceduralMeshfromStaticMeshComponent (Variables|Default|GetMesh2Slice) 0 (Variables|Default|GetProceduralMesh) true))

(fn ConstructionScript)