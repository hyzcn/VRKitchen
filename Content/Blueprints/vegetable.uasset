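; Vegetable actor that turns its static mesh into a physics-simulated procedural mesh with collision and a dynamic material, apparently intended for slicing and cooking.
; Tick calls CookVeggie while IsOnFire is set, but that function is empty, with its HowCooked material increment left disconnected.
; The mesh-slicing logic is also unwired.
; GetLogString reads HowCooked, but its string-building node is unused.
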(event EventBeginPlay
  (bind _proceduralmesh (Variables|Default|GetProceduralMesh))
  (bind _staticmesh (Variables|Default|GetStaticMesh))
  (Class|KismetProceduralMeshLibrary|CopyProceduralMeshfromStaticMeshComponent _staticmesh 0 _proceduralmesh true)
  (Physics|SetSimulatePhysics _proceduralmesh true)
  (Rendering|Material|CreateDynamicMaterialInstance (Variables|Default|GetProceduralMesh) 0 (Rendering|Material|GetMaterial _staticmesh 0) :!class /Script/Engine.PrimitiveComponent))

(event Collision|EventActorBeginOverlap
  (params (OtherActor :type Actor%20Object%20Reference)))

(event EventTick
  (params (DeltaSeconds :type Float%20%28single-precision%29))
  (if (Variables|Default|GetIsOnFire)
    (CallFunction|CookVeggie)))

(fn ConstructionScript
  (|CallParentFunction))

(fn CookVeggie)

(fn GetLogString
  (bind _asmaterial_instance_dynamic (Utilities|Casting|CastToMaterialInstanceDynamic (Rendering|Material|GetMaterial (Variables|Default|GetProceduralMesh) 0)))
  (bind _returnvalue (Rendering|Material|GetScalarParameterValue _asmaterial_instance_dynamic "HowCooked" :!class /Script/Engine.MaterialInstanceDynamic))
  (return))