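; Knife actor that slices any procedural mesh its CutMesh component overlaps.
; The cut plane takes its position and normal from the Cutnormal component, and the slice creates a second half with a Metal_Panel cap on the cut face.
; The new half simulates physics and gets a dynamic instance of the original's first material.
; Overlaps with other component types only print a debug message.
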(event OnComponentHit(StaticMesh)
  (params (HitComponent :type Primitive%20Component%20Object%20Reference) (OtherActor :type Actor%20Object%20Reference) (OtherComp :type Primitive%20Component%20Object%20Reference) (NormalImpulse :type Vector :default "0, 0, 0") (Hit :type Hit%20Result%20Structure%20%28by%20ref%29)))

(event OnComponentBeginOverlap(CutMesh)
  (params (OverlappedComponent :type Primitive%20Component%20Object%20Reference) (OtherActor :type Actor%20Object%20Reference) (OtherComp :type Primitive%20Component%20Object%20Reference) (OtherBodyIndex :type Integer) (bFromSweep :type Boolean) (SweepResult :type Hit%20Result%20Structure%20%28by%20ref%29))
  (bind _cutnormal (Variables|Default|GetCutnormal))
  (bind _asprocedural_mesh_component (Utilities|Casting|CastToProceduralMeshComponent OtherComp)
    (:then
      (bind _outotherhalfprocmesh (Class|KismetProceduralMeshLibrary|SliceProceduralMesh _asprocedural_mesh_component (Transformation|GetWorldLocation _cutnormal) (Math|Vector|GetForwardVector _cutnormal) true "CreateNewSectionForCap" "/Game/Assets/VRFancyKitchen/Metal_Panel.Metal_Panel"))
      (Physics|SetSimulatePhysics _outotherhalfprocmesh true)
      (Rendering|Material|CreateDynamicMaterialInstance _outotherhalfprocmesh 0 (Rendering|Material|GetMaterial _asprocedural_mesh_component 0) :!class /Script/Engine.PrimitiveComponent))
    (:CastFailed
      (Development|PrintString "Nocut"))))

(event EventBeginPlay)

(event Collision|EventActorBeginOverlap
  (params (OtherActor :type Actor%20Object%20Reference)))

(event EventTick
  (params (DeltaSeconds :type Float%20%28single-precision%29)))

(fn ConstructionScript
  (|CallParentFunction))