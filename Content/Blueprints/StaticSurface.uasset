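; StaticSurface is an actor representing a surface, such as a table, that tracks which objects are on it.
; Overlap begin and end events on its SurfaceArea component add and remove actors in the ObjectsOnSurface list.
; GetLogString builds a text summary of that list from the IDs of actors implementing InteractableInterface, while GetID returns the surface's own ID.
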(event OnComponentBeginOverlap(SurfaceArea)
  (params (OverlappedComponent :type Primitive%20Component%20Object%20Reference) (OtherActor :type Actor%20Object%20Reference) (OtherComp :type Primitive%20Component%20Object%20Reference) (OtherBodyIndex :type Integer) (bFromSweep :type Boolean) (SweepResult :type Hit%20Result%20Structure%20%28by%20ref%29))
  (Utilities|Array|Add (Variables|Default|GetObjectsOnSurface) OtherActor))

(event OnComponentEndOverlap(SurfaceArea)
  (params (OverlappedComponent :type Primitive%20Component%20Object%20Reference) (OtherActor :type Actor%20Object%20Reference) (OtherComp :type Primitive%20Component%20Object%20Reference) (OtherBodyIndex :type Integer))
  (Utilities|Array|RemoveItem (Variables|Default|GetObjectsOnSurface) OtherActor))

(event EventBeginPlay)

(event Collision|EventActorBeginOverlap
  (params (OtherActor :type Actor%20Object%20Reference)))

(event EventTick
  (params (DeltaSeconds :type Float%20%28single-precision%29)))

(fn ConstructionScript)

(fn GetID
  (return (Variables|Default|GetID)))

(fn GetLogString
  (LocalVariables|SetResultString (Utilities|String|Append "" "ObjectsOnTable: " "{"))
  (for _array_element (Variables|Default|GetObjectsOnSurface)
    (if (Utilities|DoesObjectImplementInterface _array_element "/Script/unreal_icra.InteractableInterface")
      (bind _returnvalue (Class|InteractableInterface|GetID(Message) _array_element))
      (LocalVariables|SetResultString (Utilities|String|Append (LocalVariables|GetResultString) _returnvalue ", "))))
  (bind _output_get (LocalVariables|SetResultString (Utilities|String|Append (LocalVariables|GetResultString) "}; ")))
  (return _output_get))