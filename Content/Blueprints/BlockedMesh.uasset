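; BlockedMesh is an actor that cuts its static mesh with two parallel planes at BeginPlay.
; It copies StaticMesh into ProceduralMesh, then slices that at Scene along CutNormal, creating a second half.
; That half is sliced again at Scene1 with the reversed normal and no new half, discarding whatever lies behind that plane.
; Cuts are capped using the last section, with a charcoal material specified.
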(event EventBeginPlay
  (bind _cutnormal (Variables|Default|GetCutNormal))
  (Class|KismetProceduralMeshLibrary|CopyProceduralMeshfromStaticMeshComponent (Variables|Default|GetStaticMesh) 0 (Variables|Default|GetProceduralMesh) false)
  (bind _outotherhalfprocmesh (Class|KismetProceduralMeshLibrary|SliceProceduralMesh (Variables|Default|GetProceduralMesh) (Transformation|GetWorldLocation (Variables|Default|GetScene)) _cutnormal true "UseLastSectionForCap" "/Game/Assets/VRFancyKitchen/_Charcoal_._Charcoal_"))
  (Class|KismetProceduralMeshLibrary|SliceProceduralMesh _outotherhalfprocmesh (Transformation|GetWorldLocation (Variables|Default|GetScene1)) (* _cutnormal -1) false "UseLastSectionForCap" "/Game/Assets/VRFancyKitchen/_Charcoal_._Charcoal_"))

(event Collision|EventActorBeginOverlap
  (params (OtherActor :type Actor%20Object%20Reference)))

(event EventTick
  (params (DeltaSeconds :type Float%20%28single-precision%29)))

(fn ConstructionScript)