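; Interactable container actor that tracks which actors are inside it and reports its contents as a log string.
; Begin and end overlap events on the Inside component add and remove actors in the ObjectsInside array.
; GetLogString joins the ID messages of contents implementing InteractableInterface and appends a hardcoded false ContainsWater field, while GetID returns the container's own ID.
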(event OnComponentBeginOverlap(Inside)
  (params (OverlappedComponent :type Primitive%20Component%20Object%20Reference) (OtherActor :type Actor%20Object%20Reference) (OtherComp :type Primitive%20Component%20Object%20Reference) (OtherBodyIndex :type Integer) (bFromSweep :type Boolean) (SweepResult :type Hit%20Result%20Structure%20%28by%20ref%29))
  (Utilities|Array|Add (Variables|Default|GetObjectsInside) OtherActor))

(event OnComponentEndOverlap(Inside)
  (params (OverlappedComponent :type Primitive%20Component%20Object%20Reference) (OtherActor :type Actor%20Object%20Reference) (OtherComp :type Primitive%20Component%20Object%20Reference) (OtherBodyIndex :type Integer))
  (Utilities|Array|RemoveItem (Variables|Default|GetObjectsInside) OtherActor))

(event EventBeginPlay)

(event Collision|EventActorBeginOverlap
  (params (OtherActor :type Actor%20Object%20Reference)))

(event EventTick
  (params (DeltaSeconds :type Float%20%28single-precision%29)))

(fn ConstructionScript
  (|CallParentFunction))

(fn GetLogString
  (LocalVariables|SetResultString "ObjectsInside: {")
  (for _array_element (Variables|Default|GetObjectsInside)
    (if (Utilities|DoesObjectImplementInterface _array_element "/Script/unreal_icra.InteractableInterface")
      (bind _returnvalue (Class|InteractableInterface|GetID(Message) _array_element))
      (LocalVariables|SetResultString (Utilities|String|Append (LocalVariables|GetResultString) _returnvalue ", "))))
  (return (Utilities|String|Append (LocalVariables|GetResultString) "};  ContainsWater: false; ")))

(fn GetID
  (return (Variables|Default|GetID)))