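; Kettle actor that heats up while on fire and starts boiling.
; Tick adds delta time to Temperature while IsOnFire is set; past a threshold it latches IsBoiling, activates two particle systems and prints a debug message.
; BeginPlay resets Temperature, EndPlay prints it, and GetLogString reports the boiling state.
; An older Timeline-based boil check is left disconnected, and GetID's result is unused in the log string.
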(event EventBeginPlay
  (Variables|Default|SetTemperature 0.0))

(event Collision|EventActorBeginOverlap
  (params (OtherActor :type Actor%20Object%20Reference)))

(event EventTick
  (params (DeltaSeconds :type Float%20%28single-precision%29))
  (if (Variables|Default|GetIsOnFire)
    (bind _output_get (Variables|Default|SetTemperature (+ (Variables|Default|GetTemperature) DeltaSeconds)))
    (if (and (> _output_get 1e+01) (not (Variables|Default|GetIsBoiling)))
      (Variables|Default|SetIsBoiling true)
      (Components|Activation|Activate (Variables|Default|GetParticleSystem) false)
      (Development|PrintString "Yes")
      (Components|Activation|Activate (Variables|Default|GetParticleSystem1) false))))

(event EventEndPlay
  (params (EndPlayReason :type EEndPlayReason%20Enum :default "Destroyed"))
  (Development|PrintString (Utilities|String|ToString(Float) (Variables|Default|GetTemperature))))

(fn ConstructionScript
  (|CallParentFunction))

(fn GetLogString
  (return (Utilities|String|Append "" "IsBoiling: " (Utilities|String|ToString(Boolean) (Variables|Default|GetIsBoiling)) "; ")))

(fn GetID
  (return (Variables|Default|GetID)))